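; Stabilizer is a component that damps the motion of the physics primitive it is attached to, acting like a fin that resists sideways slip.
; Each tick it samples the parent's velocity at its own world location.
; It applies a delta-time-scaled impulse there, combining light drag against the full velocity with much stronger resistance along its right vector, so placement and rotation determine the effect.
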(event `self.ReceiveTick`
  (params (DeltaSeconds :type "Float (single-precision)"))
  (bind _returnvalue (`self.K2_GetComponentLocation`))
  (bind _returnvalue_2 (`KismetMathLibrary.GetRightVector` (`self.K2_GetComponentRotation`)))
  (bind _asprimitive_component (cast `PrimitiveComponent` (`self.GetAttachParent`)))
  (bind _returnvalue_3 (`PrimitiveComponent.GetPhysicsLinearVelocityAtPoint` _asprimitive_component _returnvalue "None"))
  (`PrimitiveComponent.AddImpulseAtLocation` _asprimitive_component (* (+ (* _returnvalue_3 -5.0) (* _returnvalue_2 (* (`KismetMathLibrary.Dot_VectorVector` _returnvalue_3 _returnvalue_2) -200.0))) (`GameplayStatics.GetWorldDeltaSeconds`)) _returnvalue "None"))
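; PitArea_Blueprint is a pit zone actor that repairs an F_Ship_BP ship when the ship overlaps it.
; Each overlap begin lowers ShipDamage by a fixed step, only if the result stays non-negative.
; The new value is copied to CurrentShipDamage on the MyPlayerController cached at BeginPlay.
; A short Delay ends the chain with nothing after it, so repair does not repeat during a continuous overlap.
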(event `self.ReceiveBeginPlay`
  (bind _asmy_player_controller (cast `/Game/Blueprints/MyPlayerController` (`GameplayStatics.GetPlayerController` 0)))
  (set `self.ControllerReference` _asmy_player_controller))

(event `self.ReceiveActorBeginOverlap`
  (params (OtherActor :type "Actor Object Reference"))
  (bind _asf_ship_bp (cast `/Game/Blueprints/Model/F_Ship_BP` OtherActor))
  (bind _returnvalue (- (`/Game/Blueprints/Model/F_Ship_BP.ShipDamage` _asf_ship_bp) 2))
  (if (>= _returnvalue 0)
    (bind _output_get (set `/Game/Blueprints/Model/F_Ship_BP.ShipDamage` _returnvalue _asf_ship_bp))
    (set `/Game/Blueprints/MyPlayerController.CurrentShipDamage` _output_get (`self.ControllerReference`))
    (`KismetSystemLibrary.Delay` 0.2)))

(fn `UserConstructionScript`)
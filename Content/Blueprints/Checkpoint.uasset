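; Checkpoint actor that registers when the player ship passes through it in the correct direction.
; When the trigger overlap with an F_Ship_BP ends, it dots the ship's velocity with the arrow component's forward vector to confirm forward travel.
; A valid pass fires CheckpointCleared with its checkpoint number, hides the particle effect and disables further overlap events on the trigger.
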(event `self.Trigger.OnComponentEndOverlap`
  (params (OverlappedComponent :type "PrimitiveComponent Object Reference") (OtherActor :type "Actor Object Reference") (OtherComp :type "PrimitiveComponent Object Reference") (OtherBodyIndex :type Integer))
  ;[1 1 1] Checkpoint System Cleared when Overlaping ends
  (bind _asf_ship_bp (cast `/Game/Blueprints/Model/F_Ship_BP` OtherActor))
  (if (> (`KismetMathLibrary.Dot_VectorVector` (`self.GetVelocity` _asf_ship_bp) (`KismetMathLibrary.Conv_RotatorToVector` (`SceneComponent.K2_GetComponentRotation` (`self.Arrow`)))) 0.0)
    (`self.CheckpointCleared` (`self.CheckpointNumber`))
    (`SceneComponent.SetHiddenInGame` (`self.ParticleSystem`) true false)
    (set `PrimitiveComponent.bGenerateOverlapEvents` false (`self.Trigger`))))

(fn `UserConstructionScript`)